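; BP_MetalDoor is a lockable metal door that opens and closes, requiring a lockpicking minigame while locked.
; OpenDoor on a locked door spawns Picklock_Minigame below the world origin, whose OnLockPicked event unlocks it with a sound.
; When unlocked, a DoOnce-gated FlipFlop plays or reverses a timeline that swings Arrow1's yaw.
; A sphere overlap shows or hides a widget for the first-person character.
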(event `Open Door`
  ;[0.05098 0.05098 0.05098] Picklocking to appear on door and trigger opening the door ("unlocking")
  (if (`self.IsLocked`)
    (bind _returnvalue (`|SpawnActorFromClass` "/Game/PickLocking/Picklock_Minigame.Picklock_Minigame_C" (`KismetMathLibrary.MakeTransform` (0.0 0.0 -2000.0)) "Undefined" "MultiplyWithRoot" null null))
    (add `/Game/PickLocking/Picklock_Minigame.OnLockPicked` _returnvalue (delegate `OnLockPicked`))
    (else
      ;;[0.05098 0.05098 0.05098] Open/Close Door Timeline
      (`/Engine/EditorBlueprintResources/StandardMacros.DoOnce` false :!label _label
        (:`Completed`
          (`GameplayStatics.PlaySound2D` "/Game/Sounds/OpenMetal_Door.OpenMetal_Door" 1.0 1.0 0.0 null null)
          (`/Engine/EditorBlueprintResources/StandardMacros.FlipFlop`
            (:`A`
              (bind (_direction _doorfloat) (`Timeline|OpenDoor Timeline` :!via `PlayFromStart` :!label _label_2)
                (:`Update`
                  (`SceneComponent.K2_SetRelativeRotation` (`self.Arrow1`) (`KismetMathLibrary.MakeRotator` 0.0 0.0 (`KismetMathLibrary.Lerp` 0.0 90.0 _doorfloat)) false false))
                (:`Finished`
                  (goto _label :!via `Reset`))))
            (:`B`
              (goto _label_2 :!via `Reverse`))))))))

(event `OnLockPicked`
  ;[0.05098 0.05098 0.05098] Picklocking to appear on door and trigger opening the door ("unlocking")
  (set `self.IsLocked` false)
  (`GameplayStatics.PlaySound2D` "/Game/Sounds/MetalDoor_PickLock.MetalDoor_PickLock" 3.0 1.0 0.0 null null))

(event `self.Sphere.OnComponentBeginOverlap`
  (params (OverlappedComponent :type "PrimitiveComponent Object Reference") (OtherActor :type "Actor Object Reference") (OtherComp :type "PrimitiveComponent Object Reference") (OtherBodyIndex :type Integer) (bFromSweep :type Boolean) (SweepResult :type "HitResult Structure (by ref)"))
  (cast `/Game/FirstPerson/Blueprints/BP_FirstPersonCharacter` OtherActor)
  (`SceneComponent.SetVisibility` (`self.Widget`) true false))

(event `self.Sphere.OnComponentEndOverlap`
  (params (OverlappedComponent :type "PrimitiveComponent Object Reference") (OtherActor :type "Actor Object Reference") (OtherComp :type "PrimitiveComponent Object Reference") (OtherBodyIndex :type Integer))
  (cast `/Game/FirstPerson/Blueprints/BP_FirstPersonCharacter` OtherActor)
  (`SceneComponent.SetVisibility` (`self.Widget`) false false))

(fn `UserConstructionScript`)