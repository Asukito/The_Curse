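; Door actor that swings open and closed, with an optional lock that is opened through a picklocking minigame.
; OpenDoor, when locked, spawns a Picklock_Minigame far below the world origin and binds its OnLockPicked event, which unlocks the door and plays an unlock sound.
; When unlocked, each call alternates via a FlipFlop between playing and reversing a timeline that lerps the door's yaw through a quarter turn.
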(event `Open Door`
  ;[0.05098 0.05098 0.05098] Picklocking to appear on door and trigger opening the door ("unlocking")
  (if (`self.IsLocked`)
    (bind _returnvalue (`|SpawnActorFromClass` "/Game/PickLocking/Picklock_Minigame.Picklock_Minigame_C" (`KismetMathLibrary.MakeTransform` (0.0 0.0 -2000.0)) "Undefined" "MultiplyWithRoot" null null))
    (add `/Game/PickLocking/Picklock_Minigame.OnLockPicked` _returnvalue (delegate `OnLockPicked`))
    (else
      ;;[0.05098 0.05098 0.05098] Open/Close Door Timeline
      (`/Engine/EditorBlueprintResources/StandardMacros.FlipFlop`
        (:`A`
          (bind (_direction _doorfloat) (`Timeline|OpenDoor Timeline` :!via `PlayFromStart` :!label _label)
            (:`Update`
              (`SceneComponent.K2_SetRelativeRotation` (`self.Door`) (`KismetMathLibrary.MakeRotator` 0.0 0.0 (`KismetMathLibrary.Lerp` 0.0 90.0 _doorfloat)) false false))))
        (:`B`
          (goto _label :!via `Reverse`))))))

(event `OnLockPicked`
  ;[0.05098 0.05098 0.05098] Picklocking to appear on door and trigger opening the door ("unlocking")
  (set `self.IsLocked` false)
  (`GameplayStatics.PlaySound2D` "/Game/Sounds/494128__wlabarron__hotel-room-door-unlocking.494128__wlabarron__hotel-room-door-unlocking" 3.0 1.0 0.0 null null))

(fn `UserConstructionScript`)