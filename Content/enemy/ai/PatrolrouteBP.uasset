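; Patrol route Blueprint that supplies waypoints along a spline, apparently for enemy AI patrols.
; The patrolRoute event advances PatrolIndex by Direction and wraps it to 0 upon reaching the last spline point, so that point is skipped.
; Direction is set to 1 when a step lands on 0, and no logic here reverses it.
; GetSplineLocation returns the world location of the current point.
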(event `patrolRoute`
  (bind _output_get (set `self.PatrolIndex` (+ (`self.PatrolIndex`) (`self.Direction`))))
  (if (== _output_get (- (`SplineComponent.GetNumberOfSplinePoints` (`self.Patrol`)) 1))
    (set `self.PatrolIndex` 0)
    (elif (== (`self.PatrolIndex`) 0)
      (set `self.Direction` 1))))

(fn `GetSplineLocation`
  (returns (location :type "Vector Structure"))
  (return (`SplineComponent.GetLocationAtSplinePoint` (`self.Patrol`) (`self.PatrolIndex`) "World")))

(fn `UserConstructionScript`)